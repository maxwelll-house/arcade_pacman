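; BP_PowerPellet is the power pellet pickup that makes enemies vulnerable when the player eats it.
; A mesh overlap with BP_Player plays a sound and eaten VFX, removes the mesh and glow, then destroys the actor after a delay.
; The same overlap notifies BP_Gamemode_Gameplay to decrement the pellet count.
; It also calls POWERPELLETEATEN on every BP_Enemy_Parent found in the level.
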(event `self.SM_PowerPellet.OnComponentBeginOverlap`
  (params (OverlappedComponent :type "PrimitiveComponent Object Reference") (OtherActor :type "Actor Object Reference") (OtherComp :type "PrimitiveComponent Object Reference") (OtherBodyIndex :type Integer) (bFromSweep :type Boolean) (SweepResult :type "HitResult Structure (by ref)"))
  (cast `/Game/ArcadeClassic/Blueprints/Character/BP_Player` OtherActor)
  (`|ExecutionSequence`
    (:`then_0`
      ;[0.2199 1 0.2734] Power pellets eaten handling
      (`GameplayStatics.PlaySound2D` "/Game/ArcadeClassic/Audio/regenerate_Cue.regenerate_Cue" 1.0 1.0 0.0 null null)
      (`ActorComponent.Activate` (`self.VFX_PowerPellet_Eaten`) false)
      (`ActorComponent.K2_DestroyComponent` (`self.SM_PowerPellet`))
      (`ActorComponent.K2_DestroyComponent` (`self.VFX_PowerPellet_Glow`))
      (`KismetSystemLibrary.Delay` 5.0)
      (`self.K2_DestroyActor`))
    (:`then_1`
      ;[0.1367 1 0.3032] Game Mode BP Decrement Pellets
      (bind _asbp_gamemode_gameplay (cast `/Game/ArcadeClassic/Blueprints/Framework/BP_Gamemode_Gameplay` (`GameplayStatics.GetGameMode`)))
      (`/Game/ArcadeClassic/Blueprints/Framework/BP_Gamemode_Gameplay.ATE PELLET` _asbp_gamemode_gameplay))
    (:`then_2`
      ;[0.1362 1 0.1893] Enemies to be vulnerable
      (bind _outactors (`GameplayStatics.GetAllActorsOfClass` "/Game/ArcadeClassic/Blueprints/Character/BP_Enemy_Parent.BP_Enemy_Parent_C"))
      (`/Game/ArcadeClassic/Blueprints/Character/BP_Enemy_Parent.POWER PELLET EATEN` _outactors))))

(fn `UserConstructionScript`)
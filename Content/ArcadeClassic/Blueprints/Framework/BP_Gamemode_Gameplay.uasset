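; BP_Gamemode_Gameplay is the gameplay game mode, which runs an intro camera move when play begins.
; BeginPlay disables player input, spawns a CameraActor at a stored location and rotation, and blends the view to it over several seconds.
; A delay slightly longer than the blend then restores input and sets AllowedToMove on the BP_Player character.
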(event `self.ReceiveBeginPlay`
  (bind _returnvalue (`GameplayStatics.GetPlayerCharacter` 0))
  (`|ExecutionSequence`
    (:`then_6`
      ;[1 0.8068 0] Gameplay camera
      (`self.DisableInput` (`GameplayStatics.GetPlayerCharacter` 0) (`GameplayStatics.GetPlayerController` 0))
      (bind _returnvalue_2 (`|SpawnActorFromClass` "/Script/Engine.CameraActor" (`KismetMathLibrary.MakeTransform` (`self.Cam_Gameplay_Loc`) (`self.Cam_Gameplay_Rot`)) "Undefined" "OverrideRootScale" null null))
      (`PlayerController.SetViewTargetWithBlend` (`GameplayStatics.GetPlayerController` 0) _returnvalue_2 6.8 "VTBlend_Linear" 0.0 false)
      (`KismetSystemLibrary.Delay` 7.0)
      (`self.EnableInput` _returnvalue (`GameplayStatics.GetPlayerController` 0))
      (bind _asbp_player (cast `/Game/ArcadeClassic/Blueprints/Character/BP_Player` _returnvalue))
      (set `/Game/ArcadeClassic/Blueprints/Character/BP_Player.bAllowedToMove` true _asbp_player))))

(fn `UserConstructionScript`)